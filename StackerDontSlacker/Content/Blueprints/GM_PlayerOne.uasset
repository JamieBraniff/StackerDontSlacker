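; GM_PlayerOne is a game mode that adds and removes a second local player for couch co-op.
; Spawning sets the default pawn to BP_PlayerTwoCharacter before creating the player, and a separate event removes player index 1 without destroying its pawn.
; AdjustPlayers works as a toggle, either removing the stored Player 2 with its pawn or creating players for active platform users lacking a controller.
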(event Custom|AdjustPlayers
  (bind _player2controller (Variables|Default|GetPlayer2Controller)
    (:then
      (Class|GameplayStatics|RemovePlayer _player2controller true))
    (:else
      (Variables|Default|SetDefaultPawnClass "/Game/Blueprints/BP_PlayerTwoCharacter.BP_PlayerTwoCharacter_C")
      (bind _outusers (Class|InputDeviceLibrary|GetAllActiveUsers))
      (for _array_element _outusers
        (Utilities|IsValid (Class|GameplayStatics|GetPlayerControllerfromPlatformUser _array_element)
          (:Is%20Not%20Valid
            (bind _returnvalue (Class|GameplayStatics|CreatePlayerfromPlatformUser _array_element))
            (Variables|Default|SetPlayer2Controller _returnvalue)))))))

(event Custom|SpawnPlayer2
  (Variables|Default|SetDefaultPawnClass "/Game/Blueprints/BP_PlayerTwoCharacter.BP_PlayerTwoCharacter_C")
  (Class|GameplayStatics|CreatePlayer -1))

(event Custom|DestroyPlayer2
  (Class|GameplayStatics|RemovePlayer (Game|GetPlayerController 1) false))

(event EventBeginPlay)

(event EventTick
  (params (DeltaSeconds :type Float%20%28single-precision%29)))

(fn ConstructionScript)

(fn SpawnPlayers)