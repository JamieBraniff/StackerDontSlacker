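; Player one's Paper2D side-scrolling character, which moves horizontally, can switch to flying, and places blocks.
; Each tick it faces its travel direction and eases the camera toward the nearest point on a Bp_Camreaspline spline, detaching it during flight input.
; Place Block cycles cube, rectangle and T-block spawns at player 0's capsule; Rotate applies a stored rotation.
; Key 0 calls AdjustPlayers on GM_PlayerOne to add player two.
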(event Custom|UpdateAnimation
  ;[1 0.7403 0.1413] Update Animation when moving
  (Sprite|SetFlipbook (Variables|Default|GetSprite) (select (> (Math|Vector|VectorLength (Variables|/Script/Engine.MovementComponent|GetVelocity (Variables|Character|GetCharacterMovement))) 0.0) "/Game/Blueprints/Placeholder_assets_Sunnylandassets/PNG/sprites/player/idle/Player1Flipbook.Player1Flipbook" "/Game/Blueprints/Placeholder_assets_Sunnylandassets/PNG/sprites/player/idle/Player1Flipbook.Player1Flipbook")))

(event Custom|UpdateControlRotation
  ;[1 0.08921 0] Update Rotation of block when turning (Will change)
  (Utilities|IsValid (Pawn|GetController)
    (:Is%20Valid
      (Math|Float|CompareFloat (.X (Math|Vector|BreakVector (Variables|/Script/Engine.MovementComponent|GetVelocity (Variables|Character|GetCharacterMovement)))) 0.0
        (:>
          (Pawn|SetControlRotation (Pawn|GetController) (Math|Rotator|MakeRotator 0.0 0.0 0.0)))
        (:<
          (Pawn|SetControlRotation (Pawn|GetController) (Math|Rotator|MakeRotator 0.0 0.0 1.8e+02)))))))

(event EventBeginPlay
  (bind _returnvalue (Actor|GetActorOfClass "/Game/Camera/Bp_Camreaspline.Bp_Camreaspline_C"))
  (Variables|Default|SetCamreaRef _returnvalue))

(event EventTick
  (params (DeltaSeconds :type Float%20%28single-precision%29))
  ;[0 1 0.1843] Event Tick
  (CallFunction|UpdateAnimation)
  (CallFunction|UpdateControlRotation)
  ;[0 1 0.1843] Move Camera-EventTick
  (Transformation|SetWorldLocation (Variables|Default|GetCamera) (Math|Interpolation|VInterpTo (Transformation|GetWorldLocation (Variables|Default|GetCamera)) (Spline|FindLocationClosesttoWorldLocation (Variables|/Game/Camera/Bp_Camreaspline.Bp_Camreaspline_C|GetSpline (Variables|Default|GetCamreaRef)) (Transformation|GetActorLocation) "World") (Utilities|Time|GetWorldDeltaSeconds) 2.0) false false))

(event Input|ActionEvents|InputActionFly
  (params (Key :type Key%20Structure :default "None"))
  (:Pressed
    (Pawn|Components|CharacterMovement|SetMovementMode (Variables|Character|GetCharacterMovement) "MOVE_Flying" 0)))

(event Input|ActionEvents|InputActionPlaceBlock
  (params (Key :type Key%20Structure :default "None"))
  ;[0.9614 1 0.2164] Spawn different blocks in order range
  (:Pressed
    (if (Variables|Default|GetBlock%201)
      (Game|SpawnActorfromClass "/Game/Blueprints/Jamie/Cube_Block.Cube_Block_C" (Math|Transform|MakeTransform (Transformation|GetWorldLocation (Variables|/Script/Engine.Character|GetCapsuleComponent (Game|GetPlayerCharacter 0))) "0, 0, 0" "1.000000,1.000000,1.000000") "AdjustIfPossibleButAlwaysSpawn" "MultiplyWithRoot" 0 0)
      (Variables|Default|SetBlock%201 false)
      (Variables|Default|SetBlock%202 true)
      (elif (Variables|Default|GetBlock%202)
        (Game|SpawnActorfromClass "/Game/Blueprints/Jamie/Rectangle_Block.Rectangle_Block_C" (Math|Transform|MakeTransform (Transformation|GetWorldLocation (Variables|/Script/Engine.Character|GetCapsuleComponent (Game|GetPlayerCharacter 0))) "0, 0, 0" "1.000000,1.000000,1.000000") "AdjustIfPossibleButAlwaysSpawn" "MultiplyWithRoot" 0 0)
        (Variables|Default|SetBlock%202 false)
        (Variables|Default|SetBlock%203 true)
        (elif (Variables|Default|GetBlock%203)
          (Game|SpawnActorfromClass "/Game/Blueprints/Jamie/T-Block.T-Block_C" (Math|Transform|MakeTransform (Transformation|GetWorldLocation (Variables|/Script/Engine.Character|GetCapsuleComponent (Game|GetPlayerCharacter 0))) "0, 0, 0" "1.000000,1.000000,1.000000") "AdjustIfPossibleButAlwaysSpawn" "MultiplyWithRoot" 0 0)
          (Variables|Default|SetBlock%203 false)
          (Variables|Default|SetBlock%201 true))))))

(event Input|ActionEvents|InputActionRotate
  (params (Key :type Key%20Structure :default "None"))
  (:Pressed
    (Utilities|FlowControl|Sequence
      (:then_0
        (Transformation|SetActorRotation (Variables|Default|GetNew%20Rotate))))))

(event Input|AxisEvents|InputAxisMoveRight
  (params (AxisValue :type Float%20%28single-precision%29))
  ;[1 0.5084 0.03639] Movement Controls
  (Pawn|Input|AddMovementInput "1.000000,0.000000,0.000000" AxisValue false))

(event Input|AxisEvents|InputAxisUp/Down
  (params (AxisValue :type Float%20%28single-precision%29))
  (if (Class|NavMovementComponent|IsFlying (Variables|Character|GetCharacterMovement))
    (Pawn|Input|AddMovementInput (Transformation|GetActorUpVector (Pawn|GetController)) AxisValue false)
    (Transformation|DetachFromComponent (Variables|Default|GetCamera) "KeepWorld" "KeepWorld" "KeepWorld" true)))

(event Input|KeyboardEvents|0
  (params (Key :type Key%20Structure :default "None"))
  ;[1 1 1] Add player 2
  (:Pressed
    (bind _asgm_player_one (Utilities|Casting|CastToGM_PlayerOne (Game|GetGameMode)))
    (Default|AdjustPlayers _asgm_player_one)))

(fn ConstructionScript)